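; Base enemy Blueprint that wanders the map, chases and attacks the player on sight, and ragdolls when its health runs out.
; A delayed AIMoveTo loop picks random navigable points until PawnSensing spots the cached player reference.
; A successful chase plays the attack animation and damages the player regardless of the sphere overlap result.
; A failed chase resumes wandering after a retriggerable delay.
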(event `MoveAroundMap`
  ;[1 0.1448 0.6305] Random Movement
  (bind _randomlocation (`NavigationSystemV1.K2_GetRandomLocationInNavigableRadius` (`self.K2_GetActorLocation`) 1000.0 null null :!label _label))
  (`|AIMoveTo` self _randomlocation null
    (:`then`
      (`KismetSystemLibrary.Delay` (`KismetMathLibrary.RandomFloatInRange` 0.5 4.0))
      (if (not (`self.SeePlayer`))
        (goto _label)))))

(event `self.ReceiveBeginPlay`
  ;[1 0.1448 0.6305] Reference to character
  (bind _asbp_player_base (cast `/Game/Marcin/Player/PlayerV1/BP_PlayerBase` (`GameplayStatics.GetPlayerCharacter` 0) :!label _label_2)
    (:`then`
      (set `self.As BP Player Base` _asbp_player_base)
      (goto _label))
    (:`CastFailed`
      (`KismetSystemLibrary.Delay` 0.2)
      (goto _label_2))))

(event `self.ReceiveAnyDamage`
  (params (Damage :type "Float (single-precision)") (DamageType :type "DamageType Object Reference") (InstigatedBy :type "Controller Object Reference") (DamageCauser :type "Actor Object Reference"))
  ;[1 0.1448 0.6305] Getting Hit and die
  (bind _output_get (set `self.HealthPoints` (- (`self.HealthPoints`) Damage)))
  (if (<= _output_get 0)
    (`self.EnemyDeath`)))

(event `self.PawnSensing.OnSeePawn`
  (params (Pawn :type "Pawn Object Reference"))
  (bind _as_bp_player_base (`self.As BP Player Base`))
  ;[1 0.1448 0.6305] AI Goni gracza
  (if (== Pawn _as_bp_player_base)
    (set `self.SeePlayer` true)
    (`|AIMoveTo` self (0.0 0.0 0.0) _as_bp_player_base 200.0
      (:`OnSuccess`
        (`self.AttackPlayer`))
      (:`OnFail`
        (`KismetSystemLibrary.RetriggerableDelay` 3.0)
        (set `self.SeePlayer` false)
        (`self.MoveAroundMap`)))))

(event `AttackPlayer`
  ;[1 0.1448 0.6305] Atak na gracza
  (`SkeletalMeshComponent.PlayAnimation` (`self.Mesh`) (`self.AttackAnim`) false)
  (`KismetSystemLibrary.SphereOverlapActors` (`SceneComponent.K2_GetComponentLocation` (`self.Sphere`)) 100.0 (`|MakeArray` "ObjectTypeQuery3" :!type "EObjectTypeQuery Enum") "/Game/Marcin/Player/PlayerV1/BP_PlayerBase.BP_PlayerBase_C")
  (`GameplayStatics.ApplyDamage` (`self.As BP Player Base`) (`self.Damage`) null self))

(fn `EnemyDeath`
  (`CharacterMovementComponent.DisableMovement` (`self.CharacterMovement`))
  (`PrimitiveComponent.SetSimulatePhysics` (`self.Mesh`) true)
  (`PrimitiveComponent.SetCollisionProfileName` (`self.Mesh`) "Ragdoll" true)
  (`PrimitiveComponent.SetCollisionEnabled` (`self.CapsuleComponent`) "NoCollision"))

(fn `UserConstructionScript`
  (`parent.UserConstructionScript`))