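; Base enemy character for wave combat, branching by type into regular enemy, boss, or placeholder healer that only plays a casting animation.
; Tick billboards the health bar and chases the player until in range, where an attack montage notify applies sphere-checked damage.
; Regular enemies report arriving at the boss to the GameMode; the boss's ArmyIsReady montages trigger its attack order.
; Death ragdolls the body, updates the kill count and advances the wave when none remain.
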(event `self.ReceiveBeginPlay`
  (bind _mesh (`self.Mesh`))
  ;[1 1 1] Setup na poczatku
  ;;[1 0.1448 0.6305] Reference to character
  (bind _asbp_player_base_v3 (cast `/Game/Marcin/Player/BP_PlayerBaseV3` (`GameplayStatics.GetPlayerCharacter` 0) :!label _label)
    (:`then`
      (set `self.As BP Player Base` _asbp_player_base_v3)
      ;;[1 0.1448 0.6305] Enemy movement + Game Mode ref
      (set `CharacterMovementComponent.MaxWalkSpeed` (`self.Walk Speed`) (`self.CharacterMovement`))
      (bind _gamemod (message `/Game/Marcin/Blueprint/BPI_GameModeV2.getGameModeRef` (`GameplayStatics.GetGameMode`)))
      (set `self.Game Mode` _gamemod)
      (bind _enemyref (`/Game/Marcin/Enemy/BPI_Enemy.getEnemyRef`))
      (set `self.Enemy Ref` _enemyref)
      ;;[1 0.1448 0.6305] Animacja spawnowania
      (`SkeletalMeshComponent.PlayAnimation` _mesh (`self.spawnAnim`) false)
      (`KismetSystemLibrary.Delay` 1.3)
      (`SkeletalMeshComponent.SetAnimationMode` _mesh "AnimationBlueprint" false)
      ;;[1 0.1448 0.6305] Aktywuje Pawn Sensing
      (`PawnSensingComponent.SetSensingUpdatesEnabled` (`self.PawnSensing`) true)
      ;;[1 0.1448 0.6305] Sets Default Chase Target
      (set `self.TargetToMoveTo` (`self.As BP Player Base`))
      ;[1 1 1] Spawnowanie - rozdzial dla roznych kategorii
      (switch `/Game/Marcin/E_EnemyType` (`self.EnemyType`)
        (:`NewEnumerator0`
          ;[1 1 1] BOSS
          (set `self.isBOSS` true)
          (set `self.TargetToMoveTo` self)
          (`self.Be Bossy`))
        (:`NewEnumerator1`
          ;[1 1 1] HEALER
          (set `self.isHealer` true))))
    (:`CastFailed`
      (`KismetSystemLibrary.Delay` 0.2)
      (goto _label))))

(event `self.CapsuleComponent.OnBeginCursorOver`
  (params (TouchedComponent :type "PrimitiveComponent Object Reference"))
  ;[1 0.1448 0.6305] Outline
  (`PrimitiveComponent.SetRenderCustomDepth` (`self.Mesh`) true))

(event `self.CapsuleComponent.OnEndCursorOver`
  (params (TouchedComponent :type "PrimitiveComponent Object Reference"))
  ;[1 0.1448 0.6305] Outline
  (`PrimitiveComponent.SetRenderCustomDepth` (`self.Mesh`) false))

(event `Be Bossy`
  ;[1 1 1] WIP - Eventy specjalne na start i w trakcie Wavea
  ;;[1 0.1448 0.6305] Boss na poczatku
  (`PawnSensingComponent.SetSensingUpdatesEnabled` (`self.PawnSensing`) false))

(event `ArmyIsReady`
  (bind _game_mode (`self.Game Mode`))
  (bind (_returnvalue_roll _returnvalue_pitch _returnvalue_yaw) (`KismetMathLibrary.BreakRotator` (`KismetMathLibrary.FindLookAtRotation` (`self.K2_GetActorLocation` self) (`self.K2_GetActorLocation` (`self.As BP Player Base`)))))
  ;[1 1 1] WIP - Eventy specjalne na start i w trakcie Wavea
  ;;[1 0.1448 0.6305] Boss na poczatku
  (`|PlayMontage` (`self.Mesh`) (`self.BossLookAround`)
    (:`OnCompleted`
      (`self.K2_SetActorRotation` self (`KismetMathLibrary.MakeRotator` 0.0 0.0 _returnvalue_yaw) false)
      (`|PlayMontage` (`self.Mesh`) (`self.BossChargeAnim`)
        (:`OnNotifyEnd`
          (`/Game/Marcin/Blueprint/GM_TopDownGameMode_MK_V2.rozkazDoAtaku` _game_mode)
          (`KismetSystemLibrary.Delay` 3.0)
          (`/Game/Marcin/Blueprint/GM_TopDownGameMode_MK_V2.showWaveEvent` _game_mode))))))

(event `StartActing`
  (params (TargetToGoTo :type "Pawn Object Reference"))
  (bind _as_bp_player_base (`self.As BP Player Base`))
  ;[1 0.1448 0.6305] Wykrycie gracza - Pawn Sensing - mogloby byc lepiej zrobione ale dziala
  (`KismetSystemLibrary.Delay` (`KismetMathLibrary.RandomFloatInRange` 0.05 2.5))
  (if (not (`self.isDead`))
    (if (`self.isBOSS`)
      (set `self.TargetToMoveTo` _as_bp_player_base)
      (if (`self.ActorHasTag` _as_bp_player_base "Player")
        (bind _output_get (set `self.PlayerPawn` _as_bp_player_base))
        (`KismetSystemLibrary.Delay` 15.0)
        (message `/Game/Marcin/Enemy/BPI_Enemy.chasePlayer` self _output_get))
      (elif (`self.isHealer`)
        (`self.BeHealer`)
        (elif (`self.ActorHasTag` TargetToGoTo "Player")
          (bind _output_get_2 (set `self.PlayerPawn` TargetToGoTo))
          (`KismetSystemLibrary.Delay` 1.3)
          (message `/Game/Marcin/Enemy/BPI_Enemy.chasePlayer` self _output_get_2))))))

(event `GoToBoss`
  (params (BossTarget :type "Pawn Object Reference"))
  (bind _returnvalue (`self.K2_GetActorLocation` BossTarget))
  ;[1 1 1] WIP - Eventy specjalne na start i w trakcie Wavea
  ;;[1 0.1448 0.6305] Enemy - move to boss
  (`KismetSystemLibrary.Delay` 1.0)
  (if (not (<= (`KismetMathLibrary.VSize` (- _returnvalue (`self.K2_GetActorLocation`))) 250.0))
    (`AITask_MoveTo.AIMoveTo` (`AIBlueprintHelperLibrary.GetAIController` self) _returnvalue null (`KismetMathLibrary.RandomFloatInRange` 300.0 1000.0) "Enable"
      (:`OnMoveFinished`
        _)))
  (`/Game/Marcin/Blueprint/GM_TopDownGameMode_MK_V2.IHaveArrived` (`self.Game Mode`)))

(event `BeHealer`
  (`KismetSystemLibrary.PrintString` "Healeruje")
  (`SkeletalMeshComponent.PlayAnimation` (`self.Mesh`) "/Game/Marcin/Enemy/AnimationsSynty/BOSS_Two_Hand_Spell_Casting_SYNTY.BOSS_Two_Hand_Spell_Casting_SYNTY" true))

(event `/Game/Marcin/Enemy/BPI_Enemy.chasePlayer`
  (params (targetPlayer :type "Pawn Object Reference"))
  ;[1 0.1448 0.6305] Chasing Player-new
  (bind _asbp_player_base_v3 (cast `/Game/Marcin/Player/BP_PlayerBaseV3` targetPlayer :!label _label_2)
    (:`then`
      (if (not (`/Game/Marcin/Player/BP_PlayerBaseV3.isDead` _asbp_player_base_v3))
        (set `self.isChasing` true)))
    (:`CastFailed`
      (`KismetSystemLibrary.Delay` 0.2)
      (goto _label_2))))

(event `CustomEvent`
  (params (targetPlayer :type "Pawn Object Reference"))
  ;[1 0 0.02677] Chasing Player - kopia zapasowa
)

(event `self.ReceiveTick`
  (params (DeltaSeconds :type "Float (single-precision)"))
  (bind _health_bar_widget (`self.Health Bar Widget`))
  (bind _returnvalue (`self.K2_GetActorLocation` (`self.TargetToMoveTo`)))
  ;[1 0.1448 0.6305] TICK
  (if (not (`self.isDead`))
    ;;[1 1 1] Health Bar
    (bind _aswb_health_bar (cast `/Game/Marcin/Blueprint/WB_HealthBar` (`WidgetComponent.GetWidget` (`self.Health Bar Widget`))))
    (`ProgressBar.SetPercent` (`/Game/Marcin/Blueprint/WB_HealthBar.HealthBar` _aswb_health_bar) (/ (`self.HealthPoints`) (`self.Max Health`)))
    (`SceneComponent.K2_SetWorldRotation` _health_bar_widget (`KismetMathLibrary.FindLookAtRotation` (`SceneComponent.K2_GetComponentLocation` _health_bar_widget) (`SceneComponent.K2_GetComponentLocation` (`PlayerCameraManager.TransformComponent` (`GameplayStatics.GetPlayerCameraManager` 0)))) false false)
    ;;[1 1 1] Move to Player
    (if (`self.isChasing`)
      (`self.MoveTo` _returnvalue)
      (if (<= (`KismetMathLibrary.VSize` (- _returnvalue (`self.K2_GetActorLocation`))) (`self.Enemy Attack Distance`))
        (set `self.isChasing` false)
        (`/Game/Marcin/Enemy/BPI_Enemy.attackPlayer` (`self.PlayerPawn`))))))

(event `self.ReceiveAnyDamage`
  (params (Damage :type "Float (single-precision)") (DamageType :type "DamageType Object Reference") (InstigatedBy :type "Controller Object Reference") (DamageCauser :type "Actor Object Reference"))
  ;[1 0.1448 0.6305] Getting Hit and die
  (if (not (`self.isBeingHit`))
    (set `self.isBeingHit` true)
    (bind _output_get (set `self.HealthPoints` (- (`self.HealthPoints`) Damage)))
    (if (<= _output_get 0)
      (`/Game/Marcin/Enemy/BPI_Enemy.Death`)
      (else
        (bind _enemyref (`self.getEnemyRef`))
        (`Controller.StopMovement` (`AIBlueprintHelperLibrary.GetAIController` _enemyref))
        (`|PlayMontage` (`self.Mesh`) (`self.gettingHitMontage`)
          (:`OnCompleted`
            _)
          (:`OnInterrupted`
            _))))
    (set `self.isBeingHit` false)
    (`/Game/Marcin/Enemy/BPI_Enemy.chasePlayer` self (`self.PlayerPawn`))))

(event `/Game/Marcin/Enemy/BPI_Enemy.Death`
  ;[1 0.1448 0.6305] EnemyDeath
  (set `self.isDead` true)
  (`CharacterMovementComponent.DisableMovement` (`self.CharacterMovement`))
  (`PrimitiveComponent.SetSimulatePhysics` (`self.Mesh`) true)
  (`PrimitiveComponent.SetCollisionProfileName` (`self.Mesh`) "Ragdoll" true)
  (`PrimitiveComponent.SetCollisionEnabled` (`self.CapsuleComponent`) "NoCollision")
  (`ActorComponent.K2_DestroyComponent` (`self.Health Bar Widget`))
  (message `/Game/Marcin/Enemy/BPI_Enemy.RemovePawn` self))

(event `/Game/Marcin/Enemy/BPI_Enemy.RemovePawn`
  (bind _game_mode (`self.Game Mode`))
  (bind _spawnedenemypawns (`/Game/Marcin/Blueprint/GM_TopDownGameMode_MK_V2.spawnedEnemyPawns` _game_mode))
  ;[1 0.1448 0.6305] Usuniecie martwego NPCa z arrayu - licznik zabitych enemich
  (`KismetArrayLibrary.Array_RemoveItem` _spawnedenemypawns self)
  (`self.EnemyDisapear`)
  (set `/Game/Marcin/Blueprint/GM_TopDownGameMode_MK_V2.eliminatedEnemies` (+ (`/Game/Marcin/Blueprint/GM_TopDownGameMode_MK_V2.eliminatedEnemies` _game_mode) 1) _game_mode)
  (`/Game/Marcin/HUD/WBP_HUD.Update eliminatedEnemies` (`/Game/Marcin/Player/BP_PlayerBaseV3.PlayerHUDRef` (`self.As BP Player Base`)))
  (if (== (`KismetArrayLibrary.Array_Length` _spawnedenemypawns) 0)
    (`KismetSystemLibrary.K2_ClearAndInvalidateTimerHandle` (`/Game/Marcin/Blueprint/GM_TopDownGameMode_MK_V2.spawnTimer` _game_mode))
    (message `/Game/Marcin/Blueprint/BPI_GameModeV2.NextWave` _game_mode)))

(event `EnemyDisapear`
  ;[1 0.1448 0.6305] Znikanie ciala
  (`KismetSystemLibrary.Delay` (`self.TimebeforeDisapearing`))
  (`self.K2_DestroyActor`))

(event `/Game/Marcin/Enemy/BPI_Enemy.attackPlayer`
  (params (targetPlayer :type "Pawn Object Reference"))
  ;[1 0.1448 0.6305] Atak na gracza
  (if (not (`self.isDead`))
    (`|PlayMontage` (`self.Mesh`) (`self.attackMontage`)
      (:`OnCompleted`
        (`KismetSystemLibrary.Delay` 0.1)
        (`/Game/Marcin/Enemy/BPI_Enemy.chasePlayer` targetPlayer :!label _label_3))
      (:`OnNotifyBegin`
        (bind (_outactors _returnvalue) (`KismetSystemLibrary.SphereOverlapActors` (`SceneComponent.K2_GetComponentLocation` (`self.Sphere`)) 100.0 (`|MakeArray` "ObjectTypeQuery3" :!type "EObjectTypeQuery Enum") (`GameplayStatics.GetObjectClass` (`self.As BP Player Base`)) (`|MakeArray` self :!type "Actor Object Reference")))
        (if _returnvalue
          (`GameplayStatics.ApplyDamage` targetPlayer (`self.Base Damage`))
          (`KismetSystemLibrary.Delay` (`self.nextAttackTime`))
          (goto _label_3)
          (else
            (`self.chasePlayer` null)))))))

(fn `BossReference`
  (returns (BossTarget :type "Pawn Object Reference"))
  (if (`|EnumEquality` (`self.EnemyType`) "NewEnumerator0")
    (return (`self.Boss Target`))))

(fn `getEnemyRef`
  (returns (EnemyRef :type "/Game/Marcin/Enemy/BP_EnemyBaseV2 Object Reference"))
  (return self))

(fn `getGameModeRef`
  (returns (GameMod :type "/Game/Marcin/Blueprint/OLD/GM_TopDownGameMode_MK Object Reference"))
  (return null))

(fn `MoveTo`
  (params (Location :type "Vector Structure"))
  (`AIBlueprintHelperLibrary.SimpleMoveToLocation` (`self.GetController`) Location))

(fn `UserConstructionScript`
  (`parent.UserConstructionScript`))